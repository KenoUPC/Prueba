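; Player character Blueprint with single-axis movement, jumping and a coin-to-diamond currency counter.
; BeginPlay adds the Enhanced Input mapping context, the move action drives movement along world X, and the jump action starts a jump.
; The Interact event passes a coin amount to SumarMonedas, which converts 100 coins into one diamond at most once per call, keeps the remainder and prints totals on screen.
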(event `self.ReceiveBeginPlay`
  (bind _asplayer_controller (cast `PlayerController` (`self.GetController`)))
  (`EnhancedInputSubsystemInterface.AddMappingContext` (pcsubsystem `EnhancedInputLocalPlayerSubsystem` _asplayer_controller) "/Game/Game/Blueprints/Character/Imputs/IMC/IMC_Default.IMC_Default" 0 (struct)))

(event `EnhancedInput|/Game/Game/Blueprints/Character/Imputs/Actions/IA_Move`
  (params (ActionValue :type "Float (double-precision)") (ElapsedSeconds :type "Float (double-precision)") (TriggeredSeconds :type "Float (double-precision)") (InputAction :type "InputAction Object Reference" :default "/Game/Game/Blueprints/Character/Imputs/Actions/IA_Move.IA_Move"))
  (:`Triggered`
    (`self.AddMovementInput` (1.0 0.0 0.0) ActionValue)))

(event `EnhancedInput|/Game/Game/Blueprints/Character/Imputs/Actions/IA_Jump`
  (params (ActionValue :type Boolean) (ElapsedSeconds :type "Float (double-precision)") (TriggeredSeconds :type "Float (double-precision)") (InputAction :type "InputAction Object Reference" :default "/Game/Game/Blueprints/Character/Imputs/Actions/IA_Jump.IA_Jump"))
  (:`Started`
    (`self.Jump`)))

(event `/Game/Game/Blueprints/Interfaces/BPI_Player.Interact`
  (params (CantidadDeMonedas :type Integer))
  (`self.SumarMonedas` CantidadDeMonedas))

(fn `SumarMonedas`
  (params (CantidadDeMonedas :type Integer))
  (bind _output_get (set `self.MonedasActuales` (+ (`self.MonedasActuales`) CantidadDeMonedas)))
  (`KismetSystemLibrary.PrintString` (`KismetStringLibrary.Conv_IntToString` _output_get))
  (if (>= _output_get 100)
    (bind _result (`/Engine/EditorBlueprintResources/StandardMacros.IncrementInt` (`self.DiamantesACtuales`))
      (:`  `
        (set `self.MonedasActuales` (- (`self.MonedasActuales`) 100))
        (`KismetSystemLibrary.PrintString` (`KismetStringLibrary.Conv_IntToString` _result) true true (struct :`R` 0.171916 :`G` 1.0 :`B` 0.141789 :`A` 1.0) 5.0)))))

(fn `UserConstructionScript`)