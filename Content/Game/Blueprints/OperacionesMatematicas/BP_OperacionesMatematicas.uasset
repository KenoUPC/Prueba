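; Learning Blueprint for basic math operations that prints results on screen.
; On BeginPlay it calls the SumaDeDosNumeros function, which adds two inputs, stores the sum and prints it.
; Unconnected graph snippets show addition, multiplication, division and subtraction of Numero1 and Numero2 into Resultado with a labelled message, but none of them run.
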(event `self.ReceiveBeginPlay`
  (bind _resultado (`self.SumaDeDosNumeros` 20 10))
  (`KismetSystemLibrary.PrintString` (`KismetStringLibrary.Conv_IntToString` _resultado) true true (struct :`R` 1.0 :`G` 0.887142 :`B` 0.030997 :`A` 1.0) 10.0))

(fn `SumaDeDosNumeros`
  (params (Num1 :type Integer) (Num2 :type Integer))
  (returns (Resultado :type Integer))
  (return (+ Num1 Num2)))

(fn `UserConstructionScript`)