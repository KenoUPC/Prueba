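; BP_BalaCañon is a cannonball projectile that flies straight along its local X axis.
; Tick adds a fixed local offset each frame without sweep, so its speed depends on frame rate and the move does no collision check.
; BeginPlay starts a delay named for destruction time, but nothing follows it, so the graph never destroys the actor.
; A disconnected debug print would show name, damage, health and armor.
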(event `self.ReceiveBeginPlay`
  (`KismetSystemLibrary.Delay` (`self.TiemproDeDestruccion`)))

(event `self.ReceiveTick`
  (params (DeltaSeconds :type "Float (single-precision)"))
  (`self.K2_AddActorLocalOffset` (5.0 0.0 0.0)))

(fn `UserConstructionScript`)