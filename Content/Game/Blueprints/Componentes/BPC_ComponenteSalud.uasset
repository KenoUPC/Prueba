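; BPC_ComponenteSalud is a health component that tracks a current life value, VidaActual.
; RestarVida subtracts damage from it and SumarVida adds healing, each printing a debug message and the new value on screen.
; Neither function clamps the result or handles death, and the event graph holds only disabled placeholder events.
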(fn `RestarVida`
  (params (`Daño` :type "Float (double-precision)"))
  (bind _output_get (set `self.VidaActual` (- (`self.VidaActual`) `Daño`)))
  (`KismetSystemLibrary.PrintString` "Se resto Vida" true true (struct :`R` 1.0 :`G` 0.158504 :`B` 0.098295 :`A` 1.0) 5.0)
  (`KismetSystemLibrary.PrintString` (`KismetStringLibrary.Conv_DoubleToString` _output_get)))

(fn `SumarVida`
  (params (VidaACurar :type "Float (double-precision)"))
  (bind _output_get (set `self.VidaActual` (+ (`self.VidaActual`) VidaACurar)))
  (`KismetSystemLibrary.PrintString` "Se sumo vida: \n")
  (`KismetSystemLibrary.PrintString` (`KismetStringLibrary.Conv_DoubleToString` _output_get)))